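; Player character for a third-person shooter, handling health, death, weapons and Enhanced Input actions.
; On possession it creates the HUD through the player controller and adds the input mapping.
; Overlapped interactables receive pickup messages; weapons attach to a hand socket, switch by ID and take matching ammo.
; Aiming drives the AnimBP and walk speed, shots route through server and owning-client events, and death calls AddKills before destroying the actor.
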(event OnComponentBeginOverlap(Box)
  (params (OverlappedComponent :type Primitive%20Component%20Object%20Reference) (OtherActor :type Actor%20Object%20Reference) (OtherComp :type Primitive%20Component%20Object%20Reference) (OtherBodyIndex :type Integer) (bFromSweep :type Boolean) (SweepResult :type Hit%20Result%20Structure%20%28by%20ref%29))
  (if (Utilities|DoesObjectImplementInterface OtherActor "/Game/TPS/Blueprints/Interfaces/BPI_Interact.BPI_Interact_C")
    (Class|BPIInteract|OnPickUp(Message) OtherActor self)))

(event Custom|Dead
  (bind _returnvalue (UserInterface|CreateWidget "/Game/TPS/Blueprints/UI/WBP_Dead.WBP_Dead_C"))
  (UserInterface|Viewport|AddtoViewport _returnvalue 0))

(event EventBeginPlay
  (bind _asabp_manny (Utilities|Casting|CastToABP_Manny (Components|SkeletalMesh|GetAnimInstance (Variables|Character|GetMesh))))
  (Variables|References|SetABP_Player _asabp_manny))

(event Game|Damage|EventAnyDamage
  (params (Damage :type Float%20%28single-precision%29) (DamageType :type Damage%20Type%20Object%20Reference) (InstigatedBy :type Controller%20Object%20Reference) (DamageCauser :type Actor%20Object%20Reference))
  (if (not (Variables|Player|GetIsDead))
    (bind _output_get (Variables|Player|SetCurrentHealth (Math|Integer|Clamp(Integer) (- (Variables|Player|GetCurrentHealth) Damage) (Variables|Player|GetHealthMin) (Variables|Player|GetHealthMax))))
    (if (<= _output_get (Variables|Player|GetHealthMin))
      (bind _asbp_ps_tps (Utilities|Casting|CastToBP_PS_TPS (Variables|Default|GetPlayerState)))
      (Default|AddKills _asbp_ps_tps)
      (Variables|Player|SetIsDead true)
      (Input|DisableInput (.AsPlayer%20Controller (Utilities|Casting|CastToPlayerController (Pawn|GetController))))
      (CallFunction|Dead)
      (Utilities|FlowControl|Delay 4.0)
      (Actor|DestroyActor))))

(event EventPossessed
  (params (NewController :type Controller%20Object%20Reference))
  ;[1 1 1] Connect to the Player Controller after Possession
  (bind _asbp_pc_tps (Utilities|Casting|CastToBP_PC_TPS NewController :!label _label)
    (:then
      (Utilities|FlowControl|DelayUntilNextTick)
      (bind _output_get (Variables|References|SetPC_TPS _asbp_pc_tps))
      (Default|CreateHUD (Variables|/Game/TPS/Blueprints/Core/BP_PC_TPS.BP_PC_TPS_C|GetBPC_UI_Manager _output_get))
      (Input|AddMappingContext (PlayerController|LocalPlayerSubsystems|GetEnhancedInputLocalPlayerSubsystem (Game|GetPlayerController 0)) "/Game/TPS/Inputs/IMC_Default.IMC_Default" 0 "(bIgnoreAllPressedKeysUntilRelease=True,bForceImmediately=False)"))
    (:CastFailed
      (Utilities|FlowControl|Delay 0.2)
      (goto _label))))

(event Custom|Shot_Server
  (params (InFired :type Boolean))
  (bind _currentweapon (Variables|Weapons|GetCurrentWeapon))
  (Utilities|IsValid _currentweapon
    (:Is%20Valid
      (Default|OnShoot _currentweapon InFired)
      (CallFunction|ShotOwning InFired))))

(event Custom|Shot_Owning
  (params (InFired :type Boolean))
  (bind _currentweapon (Variables|Weapons|GetCurrentWeapon))
  (Utilities|IsValid _currentweapon
    (:Is%20Valid
      (Default|OnShoot _currentweapon InFired))))

(event Input|EnhancedActionEvents|EnhancedInputActionIA_Shot
  (params (ActionValue :type Boolean) (ElapsedSeconds :type Float%20%28double-precision%29) (TriggeredSeconds :type Float%20%28double-precision%29) (InputAction :type Input%20Action%20Object%20Reference :default "/Game/TPS/Inputs/Actions/IA_Shot.IA_Shot"))
  (:Started
    (bind _currentweapon (Variables|Weapons|GetCurrentWeapon)
      (:then
        (if (not (Variables|/Game/TPS/Blueprints/Weapons/BP_BaseWeapon.BP_BaseWeapon_C|GetIsReload _currentweapon))
          (CallFunction|ShotServer true)))
      (:else)))
  (:Completed
    (bind _currentweapon_2 (Variables|Weapons|GetCurrentWeapon)
      (:then
        (if (not (Variables|/Game/TPS/Blueprints/Weapons/BP_BaseWeapon.BP_BaseWeapon_C|GetIsReload _currentweapon_2))
          (CallFunction|ShotServer false)))
      (:else))))

(event Input|EnhancedActionEvents|EnhancedInputActionIA_Reload
  (params (ActionValue :type Boolean) (ElapsedSeconds :type Float%20%28double-precision%29) (TriggeredSeconds :type Float%20%28double-precision%29) (InputAction :type Input%20Action%20Object%20Reference :default "/Game/TPS/Inputs/Actions/IA_Reload.IA_Reload"))
  (bind _currentweapon (Variables|Weapons|GetCurrentWeapon))
  (:Started
    (Utilities|IsValid _currentweapon
      (:Is%20Valid
        (Default|ReloadWeapon _currentweapon)))))

(event Input|EnhancedActionEvents|EnhancedInputActionIA_FirstWeapon
  (params (ActionValue :type Boolean) (ElapsedSeconds :type Float%20%28double-precision%29) (TriggeredSeconds :type Float%20%28double-precision%29) (InputAction :type Input%20Action%20Object%20Reference :default "/Game/TPS/Inputs/Actions/IA_FirstWeapon.IA_FirstWeapon"))
  (:Started
    (bind _currentweapon (Variables|Weapons|GetCurrentWeapon)
      (:then
        (if (not (Variables|/Game/TPS/Blueprints/Weapons/BP_BaseWeapon.BP_BaseWeapon_C|GetIsReload _currentweapon))
          (CallFunction|SetWeapon "NewEnumerator1")))
      (:else))))

(event Input|EnhancedActionEvents|EnhancedInputActionIA_SecondWeapon
  (params (ActionValue :type Boolean) (ElapsedSeconds :type Float%20%28double-precision%29) (TriggeredSeconds :type Float%20%28double-precision%29) (InputAction :type Input%20Action%20Object%20Reference :default "/Game/TPS/Inputs/Actions/IA_SecondWeapon.IA_SecondWeapon"))
  (:Started
    (bind _currentweapon (Variables|Weapons|GetCurrentWeapon)
      (:then
        (if (not (Variables|/Game/TPS/Blueprints/Weapons/BP_BaseWeapon.BP_BaseWeapon_C|GetIsReload _currentweapon))
          (CallFunction|SetWeapon "NewEnumerator0")))
      (:else))))

(event Input|EnhancedActionEvents|EnhancedInputActionIA_ThirdWeapon
  (params (ActionValue :type Boolean) (ElapsedSeconds :type Float%20%28double-precision%29) (TriggeredSeconds :type Float%20%28double-precision%29) (InputAction :type Input%20Action%20Object%20Reference :default "/Game/TPS/Inputs/Actions/IA_ThirdWeapon.IA_ThirdWeapon"))
  (:Started
    (bind _currentweapon (Variables|Weapons|GetCurrentWeapon)
      (:then
        (if (not (Variables|/Game/TPS/Blueprints/Weapons/BP_BaseWeapon.BP_BaseWeapon_C|GetIsReload _currentweapon))
          (CallFunction|SetWeapon "NewEnumerator3")))
      (:else))))

(event Input|EnhancedActionEvents|EnhancedInputActionIA_Aim
  (params (ActionValue :type Boolean) (ElapsedSeconds :type Float%20%28double-precision%29) (TriggeredSeconds :type Float%20%28double-precision%29) (InputAction :type Input%20Action%20Object%20Reference :default "/Game/TPS/Inputs/Actions/IA_Aim.IA_Aim"))
  (bind _abp_player (Variables|References|GetABP_Player))
  (:Started
    (Variables|/Game/TPS/Blueprints/Characters/Mannequins/Animations/ABP_Manny.ABP_Manny_C|SetAiming _abp_player true)
    (Variables|/Script/Engine.CharacterMovementComponent|SetMaxWalkSpeed (Variables|Character|GetCharacterMovement) 2.3e+02))
  (:Completed
    (Variables|/Game/TPS/Blueprints/Characters/Mannequins/Animations/ABP_Manny.ABP_Manny_C|SetAiming _abp_player false)
    (Variables|/Script/Engine.CharacterMovementComponent|SetMaxWalkSpeed (Variables|Character|GetCharacterMovement) 5e+02)))

(event Input|EnhancedActionEvents|EnhancedInputActionIA_OpenBoard
  (params (ActionValue :type Boolean) (ElapsedSeconds :type Float%20%28double-precision%29) (TriggeredSeconds :type Float%20%28double-precision%29) (InputAction :type Input%20Action%20Object%20Reference :default "/Game/TPS/Inputs/Actions/IA_OpenBoard.IA_OpenBoard"))
  (:Started
    (Default|CallOnCheckingBoard)))

(fn ConstructionScript)

(fn AttachWeapon
  (params (WeaponBase :type BP%20Base%20Weapon%20Object%20Reference))
  (Utilities|IsValid (Variables|Weapons|GetCurrentWeapon)
    (:Is%20Valid
      (Development|SetHiddeninGame (Variables|/Game/TPS/Blueprints/Weapons/BP_BaseWeapon.BP_BaseWeapon_C|GetSkeletalMesh (Variables|Weapons|GetCurrentWeapon)) true false))
    (:Is%20Not%20Valid
      _))
  (bind _output_get (Variables|Weapons|SetCurrentWeapon WeaponBase))
  (Transformation|AttachComponentToComponent _output_get (Variables|Character|GetMesh) "WeaponSocket" "SnapToTarget" "SnapToTarget" "SnapToTarget" true)
  (Utilities|Array|AddUnique (Variables|Weapons|GetWeapons) (Variables|Weapons|GetCurrentWeapon))
  (Default|OnActivated (Variables|Weapons|GetCurrentWeapon))
  (Variables|/Game/TPS/Blueprints/Characters/Mannequins/Animations/ABP_Manny.ABP_Manny_C|SetWeaponInHand (Variables|References|GetABP_Player) true))

(fn AmmoPickUp
  (params (Ammo :type BP%20Ammo%20Base%20Object%20Reference))
  (bind _currentweapon (Variables|Weapons|GetCurrentWeapon))
  (Utilities|IsValid Ammo
    (:Is%20Valid
      (Utilities|IsValid _currentweapon
        (:Is%20Valid
          (if (Utilities|Enum|Equal(Enum) (Variables|/Game/TPS/Blueprints/Ammo/BP_AmmoBase.BP_AmmoBase_C|GetWeaponID Ammo) (Variables|/Game/TPS/Blueprints/Weapons/BP_BaseWeapon.BP_BaseWeapon_C|GetWeaponID _currentweapon))
            (Default|SetAllAmmo (Variables|Weapons|GetCurrentWeapon) (Default|GetAmmo Ammo))
            (Actor|DestroyActor Ammo)
            (else
              (bind _array_element (Utilities|Array|ForEachLoopwithBreak (Variables|Weapons|GetWeapons) :!label _label)
                (:LoopBody
                  (if (Utilities|Enum|Equal(Enum) (Variables|/Game/TPS/Blueprints/Weapons/BP_BaseWeapon.BP_BaseWeapon_C|GetWeaponID _array_element) (Variables|/Game/TPS/Blueprints/Ammo/BP_AmmoBase.BP_AmmoBase_C|GetWeaponID Ammo))
                    (Default|SetAllAmmo _array_element (Default|GetAmmo Ammo))
                    (Actor|DestroyActor Ammo)
                    (goto _label Break)))))))))))

(fn SwitchingWeapon
  (params (CurrentWeapon :type BP%20Base%20Weapon%20Object%20Reference))
  (Utilities|IsValid (Variables|Weapons|GetCurrentWeapon)
    (:Is%20Valid
      (Development|SetHiddeninGame (Variables|/Game/TPS/Blueprints/Weapons/BP_BaseWeapon.BP_BaseWeapon_C|GetSkeletalMesh (Variables|Weapons|GetCurrentWeapon)) true false))
    (:Is%20Not%20Valid
      _))
  (bind _output_get (Variables|Weapons|SetCurrentWeapon CurrentWeapon))
  (Development|SetHiddeninGame (Variables|/Game/TPS/Blueprints/Weapons/BP_BaseWeapon.BP_BaseWeapon_C|GetSkeletalMesh _output_get) false false)
  (Default|OnActivated (Variables|Weapons|GetCurrentWeapon))
  (return))

(fn SetWeapon
  (params (WeaponType :type E_AmmoType%20Enum :default "NewEnumerator0"))
  (Variables|Weapons|SetWeaponType WeaponType)
  (bind _array_element (Utilities|Array|ForEachLoopwithBreak (Variables|Weapons|GetWeapons) :!label _label)
    (:LoopBody
      (Utilities|IsValid (Variables|Weapons|GetCurrentWeapon)
        (:Is%20Valid
          (if (Utilities|Enum|Equal(Enum) (Variables|/Game/TPS/Blueprints/Weapons/BP_BaseWeapon.BP_BaseWeapon_C|GetWeaponID _array_element) (Variables|Weapons|GetWeaponType))
            (if (not (Utilities|Enum|Equal(Enum) (Variables|Weapons|GetWeaponType) (Variables|/Game/TPS/Blueprints/Weapons/BP_BaseWeapon.BP_BaseWeapon_C|GetWeaponID (Variables|Weapons|GetCurrentWeapon))))
              (CallFunction|SwitchingWeapon _array_element)
              (goto _label Break))))))))