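; BPC_UI_Manager is a component on the TPS player controller that owns the player's HUD.
; On BeginPlay, for the local controller only, it replaces any existing HUD with a new WBP_HUD, broadcasts its activation and switches to game-only input with the cursor hidden.
; UpdateAmmo forwards a weapon to the HUD's weapon state widget to refresh the ammo message.
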(event Custom|CreateHUD
  (bind _returnvalue (Game|GetPlayerController 0))
  (if (Pawn|IsLocalPlayerController (.AsBP%20PC%20TPS (Utilities|Casting|CastToBP_PC_TPS (Components|GetOwner))))
    (bind _wb_hud (Variables|Default|GetWB_HUD)
      (:then
        (Widget|RemovefromParent _wb_hud))
      (:else
        _))
    (bind _returnvalue_2 (UserInterface|CreateWidget "/Game/TPS/Blueprints/UI/WBP_HUD.WBP_HUD_C" _returnvalue))
    (bind _output_get (Variables|Default|SetWB_HUD _returnvalue_2))
    (UserInterface|Viewport|AddtoViewport _output_get 0)
    (Default|CallOnHudActivated _output_get)
    (Variables|/Script/Engine.PlayerController|SetbShowMouseCursor _returnvalue false)
    (Input|SetInputModeGameOnly _returnvalue false)))

(event EventBeginPlay
  (if (Pawn|IsLocalPlayerController (.AsBP%20PC%20TPS (Utilities|Casting|CastToBP_PC_TPS (Components|GetOwner))))
    (CallFunction|CreateHUD)))

(event EventUpdateAmmo
  (params (Weapon :type BP%20Base%20Weapon%20Object%20Reference))
  (Class|BPIUI|UpdateAmmo(Message) (Variables|/Game/TPS/Blueprints/UI/WBP_HUD.WBP_HUD_C|GetWBP_WeaponState (Variables|Default|GetWB_HUD)) Weapon))