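; Spawn system component that spawns TPS player characters at team-specific spawn points.
; On BeginPlay the authority gathers all BP_PlayerSpawn actors and sorts them into Team 0 and Team 1 lists.
; A spawn request for a controller without a pawn reads the team from the PlayerState's BPC_Team component, picks a random matching point, then spawns and possesses a BP_PlayerCharacter_TPS there.
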(event Custom|Server_SpawnPlayerWithTeam
  (params (PlayerController :type Player%20Controller%20Object%20Reference))
  ;[1 1 1] Server_SpawnPlayer
  (Utilities|IsValid (Pawn|GetControlledPawn PlayerController)
    (:Is%20Not%20Valid
      (bind _spawn (CallFunction|ChooseSpawn (Default|GetTeam (Actor|GetComponentbyClass (Variables|/Script/Engine.Controller|GetPlayerState PlayerController) "/Game/TPS/Blueprints/Components/BPC_Team.BPC_Team_C"))))
      (CallFunction|Spawn _spawn PlayerController))))

(event Custom|Spawn
  (params (Spawn :type BP%20Player%20Spawn%20Object%20Reference) (PC :type Player%20Controller%20Object%20Reference))
  ;[1 1 1] Server_SpawnPlayer
  (bind _returnvalue (Game|SpawnActorfromClass "/Game/TPS/Blueprints/Characters/BP_PlayerCharacter_TPS.BP_PlayerCharacter_TPS_C" (Transformation|GetActorTransform Spawn) "AdjustIfPossibleButAlwaysSpawn" "SelectDefaultAtRuntime" PC 0))
  (Utilities|IsValid _returnvalue
    (:Is%20Valid
      (Pawn|Possess PC _returnvalue))))

(event EventBeginPlay
  ;[0.3005 0.3005 0.3005] Get All Spawn Points
  (Networking|SwitchHasAuthority
    (:Authority
      (CallFunction|GetSpawnPoints))))

(fn GetSpawnPoints
  (bind _outactors (Actor|GetAllActorsOfClass "/Game/TPS/Blueprints/PlayerSpawn/BP_PlayerSpawn.BP_PlayerSpawn_C"))
  (bind _output_get (Variables|Default|SetSpawnPoints _outactors))
  (for _array_element _output_get
    (LocalVariables|SetSpawnPoint _array_element)
    (if (== (Variables|/Game/TPS/Blueprints/PlayerSpawn/BP_PlayerSpawn.BP_PlayerSpawn_C|GetTeam _array_element) 0)
      (Utilities|Array|AddUnique (Variables|Default|GetTeam0) (LocalVariables|GetSpawnPoint))
      (else
        (Utilities|Array|AddUnique (Variables|Default|GetTeam1) (LocalVariables|GetSpawnPoint))))))

(fn ChooseSpawn
  (params (Team :type Integer))
  (if (== Team 0)
    (return (.OutItem (Utilities|Array|Random (Variables|Default|GetTeam0))))
    (else
      (return (.OutItem (Utilities|Array|Random (Variables|Default|GetTeam1)))))))