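; TPS game mode that assigns joining players to two teams and begins match setup once the required player count is connected.
; Each new controller is tracked and given the smaller team, with ties going to team 0, through the BPC_Team component on its PlayerState.
; When the count exactly matches the requirement, all controllers receive a spawn message, then after a short delay the game state adds the main board.
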(event EventHandleStartingNewPlayer
  (params (NewPlayer :type Player%20Controller%20Object%20Reference))
  (bind _asbp_pc_tps (Utilities|Casting|CastToBP_PC_TPS NewPlayer))
  (bind _output_get (Variables|Default|SetNewPC _asbp_pc_tps))
  (Utilities|Array|AddUnique (Variables|Default|GetConnectedControllers) _output_get)
  ;[1 1 1] Initial balance
  (CallFunction|CheckingBalance _output_get)
  (Utilities|CheckingNumPlayers
    (:True
      (for _array_element (Variables|Default|GetConnectedControllers)
        (Class|BPIPlayerController|PlayerSpawn(Message) _array_element))
      (Utilities|FlowControl|Delay 3.0)
      (bind _asbp_gs_tps (Utilities|Casting|CastToBP_GS_TPS (Game|GetGameState)))
      (Default|AddMainBoard _asbp_gs_tps))))

(fn ConstructionScript)

(fn GetPlayersbyTeam
  (params (Team :type Integer))
  (for _array_element (Variables|/Script/Engine.GameStateBase|GetPlayerArray (Game|GetGameState))
    (Utilities|IsValid (Actor|GetComponentbyClass _array_element "/Game/TPS/Blueprints/Components/BPC_Team.BPC_Team_C")
      (:Is%20Valid
        (if (== (Variables|/Game/TPS/Blueprints/Components/BPC_Team.BPC_Team_C|GetTeam (Actor|GetComponentbyClass _array_element "/Game/TPS/Blueprints/Components/BPC_Team.BPC_Team_C")) Team)
          (Utilities|Array|AddUnique (LocalVariables|GetTeamPlayers) _array_element)))))
  (return (LocalVariables|GetTeamPlayers)))

(fn CheckingBalance
  (params (PC :type Controller%20Object%20Reference))
  (bind _playerstate (Variables|/Script/Engine.Controller|GetPlayerState PC))
  (bind _returnvalue (Actor|GetComponentbyClass _playerstate "/Game/TPS/Blueprints/Components/BPC_Team.BPC_Team_C"))
  (if (<= (Utilities|Array|Length (CallFunction|GetPlayersbyTeam)) (Utilities|Array|Length (CallFunction|GetPlayersbyTeam 1)))
    (Default|SetTeam _returnvalue)
    (else
      (Default|SetTeam _returnvalue 1))))