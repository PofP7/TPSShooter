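; Game state for the TPS mode that runs the match countdown and builds the player scoreboard.
; A looping one-second timer decrements the match time and fires the OnEndMatch dispatcher at or below the limit, without clearing itself.
; AddMainBoard shows the main board widget with one wins row per PlayerArray entry.
; Only the last row is kept in PlayerScore, so AddKills writes kills to that row alone.
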(event Custom|StartMatchtimer
  (Utilities|Time|SetTimerbyEvent (delegate Custom|UpdateMatchTimer) 1.0 true))

(event Custom|EndMatch
  (Default|CallOnEndMatch))

(event Custom|AddMainBoard
  (bind _returnvalue (UserInterface|CreateWidget "/Game/TPS/Blueprints/UI/WBP_MainBoard.WBP_MainBoard_C"))
  (bind _output_get (Variables|Default|SetWB_MainBoard _returnvalue))
  (UserInterface|Viewport|AddtoViewport _output_get 0)
  (for _array_element (Variables|Default|GetPlayerArray)
    (bind _returnvalue_2 (UserInterface|CreateWidget "/Game/TPS/Blueprints/UI/WBP_PlayersWins.WBP_PlayersWins_C" (Game|GetPlayerController 0) 0 (Utilities|Text|ToText(String) (PlayerState|GetPlayerName _array_element))))
    (Variables|Default|SetPlayerScore _returnvalue_2)
    (Widget|Panel|AddChild (Variables|/Game/TPS/Blueprints/UI/WBP_MainBoard.WBP_MainBoard_C|GetPlayersWin (Variables|Default|GetWB_MainBoard)) _returnvalue_2)))

(event Custom|AddKills
  (params (Kill :type Integer))
  (Variables|/Game/TPS/Blueprints/UI/WBP_PlayersWins.WBP_PlayersWins_C|SetKills (Variables|Default|GetPlayerScore) Kill))

(event Custom|UpdateMatchTimer
  (bind _output_get (Variables|Default|SetMatchTimeInSeconds (- (Variables|Default|GetMatchTimeInSeconds) 1.0)))
  (if (<= _output_get (Variables|Default|GetMatchTimeLimit))
    (CallFunction|EndMatch)))

(event EventBeginPlay
  (CallFunction|StartMatchtimer))

(fn ConstructionScript)

(fn GetTimeinSeconds
  (return (Variables|Default|GetMatchTimeInSeconds)))

(fn GetMatchTimeLimit
  (return (Variables|Default|GetMatchTimeLimit)))