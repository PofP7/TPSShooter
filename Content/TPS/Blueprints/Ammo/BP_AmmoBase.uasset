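; BP_AmmoBase is a base ammo pickup actor for the TPS game, holding a weapon ID and an ammo count with getters and setters for both.
; OnPickUp checks the picking character's weapons and, for each one with a matching WeaponID, passes itself to the character's AmmoPickUp and then fires CallOnAmmoPickup.
; The loop has no early exit, so several matching weapons trigger the pickup several times.
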(event EventBeginPlay)

(event Collision|EventActorBeginOverlap
  (params (OtherActor :type Actor%20Object%20Reference)))

(event EventTick
  (params (DeltaSeconds :type Float%20%28single-precision%29)))

(event EventOnPickUp
  (params (Character :type BP%20Player%20Character%20TPS%20Object%20Reference))
  (Utilities|IsValid Character
    (:Is%20Valid
      (for _array_element (Variables|/Game/TPS/Blueprints/Characters/BP_PlayerCharacter_TPS.BP_PlayerCharacter_TPS_C|GetWeapons Character)
        (if (Utilities|Enum|Equal(Enum) (Variables|/Game/TPS/Blueprints/Weapons/BP_BaseWeapon.BP_BaseWeapon_C|GetWeaponID _array_element) (Variables|Default|GetWeaponID))
          (Default|AmmoPickUp Character self)
          (Default|CallOnAmmoPickup))))))

(fn ConstructionScript)

(fn GetAmmo
  (return (Variables|Default|GetAmmoCount)))

(fn GetAmmoType
  (return (Variables|Default|GetWeaponID)))

(fn SetAmmoType
  (params (inWeaponType :type E_AmmoType%20Enum :default "NewEnumerator0"))
  (Variables|Default|SetWeaponID inWeaponType))

(fn SetAmmo
  (params (InAmmo :type Integer))
  (Variables|Default|SetAmmoCount InAmmo))