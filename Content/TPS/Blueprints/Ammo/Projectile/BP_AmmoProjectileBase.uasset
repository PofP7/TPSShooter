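; Base ammo projectile for the TPS weapons that plays a flight sound and resolves impacts.
; On sphere hit it spawns a particle aligned to the impact normal plus a hit sound, then destroys its particle system.
; It applies damage only to hit actors implementing BPI_HealthAttributes other than its owner, crediting the owner as damage causer, then destroys itself.
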(event OnComponentHit(Sphere)
  (params (HitComponent :type Primitive%20Component%20Object%20Reference) (OtherActor :type Actor%20Object%20Reference) (OtherComp :type Primitive%20Component%20Object%20Reference) (NormalImpulse :type Vector :default "0, 0, 0") (Hit :type Hit%20Result%20Structure%20%28by%20ref%29))
  (bind (_bblockinghit _binitialoverlap _time _distance _location _impactpoint _normal _impactnormal _physmat _hitactor) (Collision|BreakHitResult Hit))
  (Variables|Default|SetHit%20Actor _hitactor)
  (Effects|SpawnEmitteratLocation (Variables|Default|GetHitParticle) _impactpoint (Math|Rotator|MakeRotfromX _impactnormal) (Variables|Default|GetScaleSpawnParticle))
  (Audio|SpawnSoundatLocation (Variables|Default|GetHitSound) _impactpoint "0, 0, 0" 1.0 1.0 0.0 0 0)
  (Components|DestroyComponent (Variables|Default|GetParticleSystem))
  (if (and (Utilities|DoesObjectImplementInterface (Variables|Default|GetHit%20Actor) "/Game/TPS/Blueprints/Interfaces/BPI_HealthAttributes.BPI_HealthAttributes_C") (not (== (Variables|Default|GetHit%20Actor) (Components|GetOwner))))
    (Game|Damage|ApplyDamage (Variables|Default|GetHit%20Actor) (Variables|Default|GetDamage) 0 (Components|GetOwner)))
  (Actor|DestroyActor))

(event EventBeginPlay
  (Components|Activation|Activate (Variables|Default|GetFlySound) true))

(event Collision|EventActorBeginOverlap
  (params (OtherActor :type Actor%20Object%20Reference)))

(event EventTick
  (params (DeltaSeconds :type Float%20%28single-precision%29)))

(fn ConstructionScript)