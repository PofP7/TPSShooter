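; BP_AmmoSpawner is a single-use spawner that places an ammo pickup in the world.
; On BeginPlay, if AmmoSpawnClass is valid, it shows its Pickup component and spawns that class slightly above its own location.
; It binds to the spawned actor's OnAmmoPickup event and destroys itself when that fires, so there is no respawn.
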(event Custom|OnSpawn
  (bind _returnvalue (Transformation|GetActorLocation))
  (if (Utilities|IsValidClass (Variables|Default|GetAmmoSpawnClass))
    (Rendering|SetVisibility (Variables|Default|GetPickup) true false)
    (bind _returnvalue_2 (Game|SpawnActorfromClass (Variables|Default|GetAmmoSpawnClass) (Math|Transform|MakeTransform (Math|Vector|MakeVector (.x _returnvalue) (.y _returnvalue) (+ (.z _returnvalue) 3e+01)) "0, 0, 0" "1.000000,1.000000,1.000000") "Undefined" "SelectDefaultAtRuntime" 0 0))
    (EventDispatchers|BindEventtoOnAmmoPickup _returnvalue_2 (delegate Custom|OnActivated))))

(event Custom|OnActivated
  (Actor|DestroyActor))

(event EventBeginPlay
  (CallFunction|OnSpawn))

(fn ConstructionScript)