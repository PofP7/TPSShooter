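; Base third-person weapon that spins as a pickup, attaches to a character lacking that WeaponID, then handles firing and reloading.
; BeginPlay loads its data table row and binds to HUD activation for ammo widget updates.
; Firing loops on a delay for auto fire, auto-reloading with a montage when the clip empties.
; A camera line trace aims each projectile spawned from the muzzle socket, with particle and sound effects.
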(event Custom|OnShoot
  (params (InFired :type Boolean))
  (bind _output_get (Variables|Default|SetButtonIsPressed InFired))
  (if _output_get
    (if (not (Variables|Default|GetShooting))
      (bind _isclipempty (CallFunction|CheckClip))
      (if _isclipempty
        (CallFunction|AutoReload)
        (else
          (Variables|Default|SetShooting true)
          (CallFunction|ShootProcess)
          (CallFunction|SpawnAmmo)
          (Utilities|FlowControl|Delay (Variables|Default|GetShootTime))
          (Variables|Default|SetShooting false)
          (if (Variables|Default|GetisAutoFire)
            (CallFunction|AutoShoot)))))))

(event Custom|OnActivated
  (Default|CallOnWeaponActivated)
  (CallFunction|UpdateAmmoWidget))

(event Custom|AutoShoot
  (if (stale Custom|OnShoot _output_get)
    (if (not (Variables|Default|GetShooting))
      (bind _isclipempty (CallFunction|CheckClip))
      (if _isclipempty
        (CallFunction|AutoReload)
        (else
          (Variables|Default|SetShooting true)
          (CallFunction|ShootProcess)
          (CallFunction|SpawnAmmo)
          (Utilities|FlowControl|Delay (Variables|Default|GetShootTime))
          (Variables|Default|SetShooting false)
          (if (Variables|Default|GetisAutoFire)
            (CallFunction|AutoShoot)))))))

(event Custom|HudActivated
  (params (HUD :type WBP%20HUD%20Object%20Reference))
  (Variables|Default|SetHUD HUD))

(event Custom|AutoReload
  (if (not (Variables|Default|GetIsReload))
    (Variables|Default|SetIsReload true)
    (bind _isnotammo (CallFunction|CheckAllAmmo))
    (if _isnotammo
      (Variables|Default|SetIsReload false)
      (else
        (CallFunction|Reload)
        (bind _ownercharacter (Variables|Default|GetOwnerCharacter)
          (:then
            (Animation|Montage|PlayMontage (Variables|/Script/Engine.Character|GetMesh _ownercharacter) "/Game/AnimStarterPack/Retargeted/Reload_Rifle_Hip_Ret_Montage.Reload_Rifle_Hip_Ret_Montage"
              (:OnCompleted
                (Variables|Default|SetIsReload false)
                (CallFunction|UpdateAmmoWidget))))
          (:else))))))

(event Custom|ReloadWeapon
  (if (not (Variables|Default|GetIsReload))
    (Variables|Default|SetIsReload true)
    (bind _isnotammo (CallFunction|CheckAllAmmo))
    (if _isnotammo
      (Variables|Default|SetIsReload false)
      (else
        (CallFunction|Reload)
        (bind _ownercharacter (Variables|Default|GetOwnerCharacter)
          (:then
            (Animation|Montage|PlayMontage (Variables|/Script/Engine.Character|GetMesh _ownercharacter) "/Game/AnimStarterPack/Retargeted/Reload_Rifle_Hip_Ret_Montage.Reload_Rifle_Hip_Ret_Montage"
              (:OnCompleted
                (Variables|Default|SetIsReload false)
                (CallFunction|UpdateAmmoWidget))))
          (:else))))))

(event EventBeginPlay
  (bind _returnvalue (Utilities|GetDataTableRow (Variables|Default|GetDT_Weapons) (Utilities|String|StringToName (Utilities|String|EnumtoString (Variables|Default|GetWeaponID))))
    (:then
      (Variables|Default|SetS_WeaponInfo _returnvalue)
      (bind _asbp_pc_tps (Utilities|Casting|CastToBP_PC_TPS (Game|GetPlayerController 0)))
      (EventDispatchers|BindEventtoOnHudActivated (Variables|/Game/TPS/Blueprints/Core/BP_PC_TPS.BP_PC_TPS_C|GetBPC_UI_Manager _asbp_pc_tps) (delegate Custom|HudActivated)))))

(event EventTick
  (params (DeltaSeconds :type Float%20%28single-precision%29))
  (if (not (Variables|Default|GetIsPickUp))
    (Transformation|AddWorldRotation (Variables|Default|GetSkeletalMesh) "0.000000,2.000000,0.000000" false false)))

(event EventOnPickUp
  (params (Character :type BP%20Player%20Character%20TPS%20Object%20Reference))
  (for _array_element (Variables|/Game/TPS/Blueprints/Characters/BP_PlayerCharacter_TPS.BP_PlayerCharacter_TPS_C|GetWeapons Character)
    (if (Utilities|Enum|Equal(Enum) (Variables|BP_BaseWeapon_C|GetWeaponID _array_element) (Variables|Default|GetWeaponID))
      (Variables|Default|SetNotPickup true)))
  (if (not (Variables|Default|GetNotPickup))
    (Variables|Default|SetIsPickUp true)
    (Collision|SetCollisionEnabled (Variables|Default|GetSkeletalMesh) "NoCollision")
    (Utilities|IsValid Character
      (:Is%20Valid
        (Default|AttachWeapon Character self)
        (bind _output_get (Variables|Default|SetOwnerCharacter Character))
        (Variables|/Game/TPS/Blueprints/Characters/BP_PlayerCharacter_TPS.BP_PlayerCharacter_TPS_C|SetWeaponType _output_get (Variables|Default|GetWeaponID))
        (if (Pawn|IsLocallyControlled _output_get)
          (CallFunction|UpdateAmmoWidget))))))

(fn ConstructionScript)

(fn CheckClip
  (return (<= (Variables|Default|GetClip) 0)))

(fn ShootProcess
  (bind _result (Math|Integer|DecrementInt (Variables|Default|GetClip))
    (:%20%20
      (bind _output_get (Variables|Default|SetClip (Math|Integer|Clamp(Integer) _result 0 (Variables|Default|GetClipSize))))
      (Variables|Default|SetS_WeaponInfo (Utilities|Struct|MakeS_Weapon (.Image (Utilities|Struct|BreakS_Weapon (Variables|Default|GetS_WeaponInfo))) _output_get (.AllAmmo (Utilities|Struct|BreakS_Weapon (Variables|Default|GetS_WeaponInfo))) 0))
      (CallFunction|UpdateAmmoWidget))))

(fn SpawnAmmo
  (bind _ownercharacter (Variables|Default|GetOwnerCharacter))
  (bind _skeletalmesh (Variables|Default|GetSkeletalMesh))
  (bind _returnvalue (Transformation|GetSocketTransform _skeletalmesh "MuzzleFlash" "RTS_World"))
  (bind _followcamera (Variables|/Script/TPS.TPSCharacter|GetFollowCamera _ownercharacter))
  (bind _returnvalue_2 (Transformation|GetWorldLocation _followcamera))
  (Utilities|IsValid _ownercharacter
    (:Is%20Valid
      (bind (_outhit _returnvalue_3) (Collision|LineTraceByChannel _returnvalue_2 (+ _returnvalue_2 (* (Math|Vector|GetForwardVector _followcamera) "5000.000000,5000.000000,5000.000000")) "TraceTypeQuery1" false 0 "None"))
      (if _returnvalue_3
        (Variables|Default|SetCurrentAmmoRotation (Math|Rotator|FindLookatRotation (.location _returnvalue) (.ImpactPoint (Collision|BreakHitResult _outhit))))
        (else
          (Variables|Default|SetCurrentAmmoRotation (.rotation _returnvalue))))
      (Game|SpawnActorfromClass (Variables|Default|GetAmmoProjectileClass) (Math|Transform|MakeTransform (.location (Transformation|GetSocketTransform (Variables|Default|GetSkeletalMesh) "MuzzleFlash" "RTS_World")) (Variables|Default|GetCurrentAmmoRotation) "1.000000,1.000000,1.000000") "Undefined" "SelectDefaultAtRuntime" (Variables|Default|GetOwnerCharacter) 0)
      (Components|Activation|Activate (Variables|Default|GetShootParticle) true)
      (Components|Activation|Activate (Variables|Default|GetShootSound) true))))

(fn CheckAllAmmo
  (return (<= (Variables|Default|GetAllAmmo) 0)))

(fn Reload
  (if (not (<= (Variables|Default|GetAllAmmo) 0))
    (bind _output_get (Variables|Default|SetAllAmmo (+ (Variables|Default|GetClip) (Variables|Default|GetAllAmmo))))
    (if (>= _output_get (Variables|Default|GetClipSize))
      (Variables|Default|SetAllAmmo (- (Variables|Default|GetAllAmmo) (Variables|Default|GetClipSize)))
      (Variables|Default|SetClip (Variables|Default|GetClipSize))
      (else
        (Variables|Default|SetClip (Variables|Default|GetAllAmmo))
        (Variables|Default|SetAllAmmo 0)))
    (Variables|Default|SetS_WeaponInfo (Utilities|Struct|MakeS_Weapon (.Image (Utilities|Struct|BreakS_Weapon (Variables|Default|GetS_WeaponInfo))) (Variables|Default|GetClip) (Variables|Default|GetAllAmmo) 0))))

(fn SetAllAmmo
  (params (AllAmmo :type Integer))
  (Variables|Default|SetAllAmmo AllAmmo)
  (bind _output_get (Variables|Default|SetAllAmmo (+ (.AllAmmo (Utilities|Struct|BreakS_Weapon (Variables|Default|GetS_WeaponInfo))) (Variables|Default|GetAllAmmo))))
  (Variables|Default|SetS_WeaponInfo (Utilities|Struct|MakeS_Weapon (.Image (Utilities|Struct|BreakS_Weapon (Variables|Default|GetS_WeaponInfo))) (.CurrentAmmoClip (Utilities|Struct|BreakS_Weapon (Variables|Default|GetS_WeaponInfo))) _output_get 0))
  (CallFunction|UpdateAmmoWidget))

(fn UpdateAmmoWidget
  (Default|UpdateWidget (Variables|/Game/TPS/Blueprints/UI/WBP_HUD.WBP_HUD_C|GetWBP_WeaponState (Variables|Default|GetHUD)) (Variables|Default|GetOwnerCharacter)))