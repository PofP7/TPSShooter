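; BP_WeaponSpawner is a TPS spawner actor that places the weapon selected by its WeaponID in the world.
; On BeginPlay it looks up the weapon class in DT_Weapons, using the ID's enum name as the row name.
; If the class is valid, it shows its Pickup component and spawns the weapon slightly above itself.
; It binds to the weapon's OnWeaponActivated dispatcher and destroys itself when that fires.
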(event Custom|OnSpawn
  (bind _returnvalue (Transformation|GetActorLocation))
  (if (Utilities|IsValidClass (Variables|Default|GetWeapon%20Class))
    (Rendering|SetVisibility (Variables|Default|GetPickup) true false)
    (bind _returnvalue_2 (Game|SpawnActorfromClass (Variables|Default|GetWeapon%20Class) (Math|Transform|MakeTransform (Math|Vector|MakeVector (.x _returnvalue) (.y _returnvalue) (+ (.z _returnvalue) 3e+01)) "0, 0, 0" "1.000000,1.000000,1.000000") "Undefined" "SelectDefaultAtRuntime" 0 0))
    (EventDispatchers|AssignOnWeaponActivated _returnvalue_2 (delegate Custom|OnWeaponActivated))))

(event Custom|OnWeaponActivated
  (Actor|DestroyActor))

(event EventBeginPlay
  (bind _returnvalue (Utilities|GetDataTableRow "/Game/TPS/Blueprints/Data/DataTables/DT_Weapons.DT_Weapons" (Utilities|String|StringToName (Utilities|String|EnumtoString (Variables|Default|GetWeaponID))))
    (:then
      (Variables|Default|SetWeapon%20Class (.WeaponClass (Utilities|Struct|BreakS_Weapon _returnvalue)))
      (CallFunction|OnSpawn))))

(fn ConstructionScript)